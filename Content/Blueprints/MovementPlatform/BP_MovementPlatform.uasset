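; BP_MovementPlatform is a platform actor meant to move between two marker components, IniPos and FinPos.
; BeginPlay caches the world locations of both markers as the start and end points.
; A Movement timeline curve drives a vector lerp that sets the actor location without sweep.
; Nothing triggers the timeline in this graph, so the movement logic never runs here.
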(event `self.ReceiveBeginPlay`
  (set `self.InitialPos` (`SceneComponent.K2_GetComponentLocation` (`self.IniPos`)))
  (set `self.FinalPos` (`SceneComponent.K2_GetComponentLocation` (`self.FinPos`))))

(fn `UserConstructionScript`)