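; BP_DisableInput is an intro trigger actor that locks player input while the Intro1 level sequence plays.
; When the third-person character overlaps its box, it sets IsPlay, disables input, restores it after a fixed delay and destroys itself.
; BeginPlay checks IsPlay once after a brief delay, so the sequence plays only if the overlap happens at level start.
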(event `self.ReceiveBeginPlay`
  (`KismetSystemLibrary.Delay` 0.05)
  (if (`self.isPlay`)
    (bind (_outactor _returnvalue) (`LevelSequencePlayer.CreateLevelSequencePlayer` "/Game/LevelSequencers/Intro1.Intro1"))
    (`MovieSceneSequencePlayer.Play` _returnvalue)))

(event `self.Box.OnComponentBeginOverlap`
  (params (OverlappedComponent :type "PrimitiveComponent Object Reference") (OtherActor :type "Actor Object Reference") (OtherComp :type "PrimitiveComponent Object Reference") (OtherBodyIndex :type Integer) (bFromSweep :type Boolean) (SweepResult :type "HitResult Structure (by ref)"))
  (bind _returnvalue (`GameplayStatics.GetPlayerController` 0))
  (bind _asbp_third_person_character (cast `/Game/ThirdPerson/Blueprints/BP_ThirdPersonCharacter` OtherActor))
  (set `self.isPlay` true)
  (`self.DisableInput` _asbp_third_person_character _returnvalue)
  (`KismetSystemLibrary.Delay` 6.6)
  (`self.EnableInput` _asbp_third_person_character _returnvalue)
  (`self.K2_DestroyActor`))

(fn `UserConstructionScript`)