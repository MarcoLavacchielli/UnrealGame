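; BP_Turret2 is a turret that tracks and fires at a BP_ThirdPersonCharacter inside its Sphere trigger.
; On overlap it stores the character, turns red and starts a looping timer that spawns BP_ABullet from BulletSpawner.
; Tick rotates the whole actor toward the stored character.
; End overlap clears the target and timer and sets a tan color through the dynamic material instance created at BeginPlay.
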(event `Change Color`
  (params (Value :type "LinearColor Structure"))
  (`MaterialInstanceDynamic.SetVectorParameterValue` (`self.MaterialRef`) "Color" Value))

(event `self.ReceiveBeginPlay`
  (bind _returnvalue (`KismetMaterialLibrary.CreateDynamicMaterialInstance` (`PrimitiveComponent.GetMaterial` (`self.StaticMesh`) 0)))
  (bind _output_get (set `self.MaterialRef` _returnvalue))
  (`PrimitiveComponent.SetMaterial` (`self.StaticMesh`) 0 _output_get))

(event `self.Sphere.OnComponentBeginOverlap`
  (params (OverlappedComponent :type "PrimitiveComponent Object Reference") (OtherActor :type "Actor Object Reference") (OtherComp :type "PrimitiveComponent Object Reference") (OtherBodyIndex :type Integer) (bFromSweep :type Boolean) (SweepResult :type "HitResult Structure (by ref)"))
  (bind _asbp_third_person_character (cast `/Game/ThirdPerson/Blueprints/BP_ThirdPersonCharacter` OtherActor))
  (set `self.As BP Third Person Character` _asbp_third_person_character)
  (`self.Change Color` (struct :`R` 1.0 :`G` 0.126976 :`A` 1.0))
  (bind _returnvalue (`KismetSystemLibrary.K2_SetTimerDelegate` (delegate `Shoot`) 0.3 true))
  (set `self.NewVar` _returnvalue))

(event `Shoot`
  (`|SpawnActorFromClass` "/Game/Blueprints/Turret/source/BP_ABullet.BP_ABullet_C" (`SceneComponent.K2_GetComponentToWorld` (`self.BulletSpawner`)) "AlwaysSpawn" "MultiplyWithRoot" null null))

(event `self.ReceiveTick`
  (params (DeltaSeconds :type "Float (single-precision)"))
  (bind _as_bp_third_person_character (`self.As BP Third Person Character`)
    (:`then`
      (bind (_returnvalue_roll _returnvalue_pitch _returnvalue_yaw) (`KismetMathLibrary.BreakRotator` (`KismetMathLibrary.FindLookAtRotation` (`self.K2_GetActorLocation`) (`self.K2_GetActorLocation` _as_bp_third_person_character))))
      (`self.K2_SetActorRotation` (`KismetMathLibrary.MakeRotator` _returnvalue_roll _returnvalue_pitch _returnvalue_yaw)))
    (:`else`)))

(event `self.Sphere.OnComponentEndOverlap`
  (params (OverlappedComponent :type "PrimitiveComponent Object Reference") (OtherActor :type "Actor Object Reference") (OtherComp :type "PrimitiveComponent Object Reference") (OtherBodyIndex :type Integer))
  (cast `/Game/ThirdPerson/Blueprints/BP_ThirdPersonCharacter` OtherActor)
  (set `self.As BP Third Person Character` null)
  (`self.Change Color` (struct :`R` 0.786458 :`G` 0.677389 :`B` 0.483233 :`A` 1.0))
  (`KismetSystemLibrary.K2_ClearAndInvalidateTimerHandle` (`self.NewVar`)))

(fn `UserConstructionScript`)