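; BP_GemSpawner is a one-shot trigger that spawns a gem for a player who is at full health.
; When a BP_ThirdPersonCharacter enters its Box, it checks that the ACHealthComponent's current health equals max health.
; On a match it spawns a BP_IndividualGem at the SpawnPoint location, plays a 2D poof sound and destroys itself.
; Entering below full health does nothing, so the spawner remains in place.
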(event `self.Box.OnComponentBeginOverlap`
  (params (OverlappedComponent :type "PrimitiveComponent Object Reference") (OtherActor :type "Actor Object Reference") (OtherComp :type "PrimitiveComponent Object Reference") (OtherBodyIndex :type Integer) (bFromSweep :type Boolean) (SweepResult :type "HitResult Structure (by ref)"))
  (bind _asbp_third_person_character (cast `/Game/ThirdPerson/Blueprints/BP_ThirdPersonCharacter` OtherActor))
  (bind _ac_healthcomponent (`/Game/ThirdPerson/Blueprints/BP_ThirdPersonCharacter.AC_HealthComponent` _asbp_third_person_character))
  (if (== (`/Game/Blueprints/ActorComponent/Components/AC_HealthComponent.CurrentHealth` _ac_healthcomponent) (`/Game/Blueprints/ActorComponent/Components/AC_HealthComponent.MaxHealth` _ac_healthcomponent))
    (`|SpawnActorFromClass` "/Game/Blueprints/Gems/BP_IndividualGem.BP_IndividualGem_C" (`KismetMathLibrary.Conv_VectorToTransform` (`SceneComponent.K2_GetComponentLocation` (`self.SpawnPoint`))) "Undefined" "MultiplyWithRoot" null null)
    (`GameplayStatics.PlaySound2D` "/Game/Sfx-Music/Y2meta_app-Magic-Poof-02-Sound-Effect-_128-kbps_.Y2meta_app-Magic-Poof-02-Sound-Effect-_128-kbps_" 2.0 1.0 0.0 null null)
    (`self.K2_DestroyActor`)))

(fn `UserConstructionScript`)