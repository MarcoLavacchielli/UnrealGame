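; Actor component that tracks an owner's health and broadcasts changes through event dispatchers.
; BeginPlay fills current health to the maximum and announces it.
; IncreaseHealth and DecreaseHealth clamp the value between zero and max, then fire OnHealthChanged.
; Healing also fires OnHealthIncrease, while damage fires OnDeath at zero or OnHealthReduce otherwise, with no guard against repeated deaths.
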(event `self.ReceiveBeginPlay`
  (bind _output_get (set `self.CurrentHealth` (`self.MaxHealth`)))
  (`self.OnHealthChanged` _output_get (`self.MaxHealth`)))

(fn `DecreaseHealth`
  (params (DmgAmount :type "Float (double-precision)"))
  (bind _output_get (set `self.CurrentHealth` (`KismetMathLibrary.FClamp` (- (`self.CurrentHealth`) DmgAmount) 0.0 (`self.MaxHealth`))))
  (`self.OnHealthChanged` _output_get (`self.MaxHealth`))
  (if (<= (`self.CurrentHealth`) 0.0)
    (`self.OnDeath`)
    (else
      (`self.OnHealthReduce`))))

(fn `IncreaseHealth`
  (params (HealAmount :type "Float (double-precision)"))
  (bind _output_get (set `self.CurrentHealth` (`KismetMathLibrary.FClamp` (+ (`self.CurrentHealth`) HealAmount) 0.0 (`self.MaxHealth`))))
  (`self.OnHealthChanged` _output_get (`self.MaxHealth`))
  (`self.OnHealthIncrease`))