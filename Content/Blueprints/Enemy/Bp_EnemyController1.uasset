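; AI controller for enemy pawns that runs the BT_Enemy1 behavior tree on possession.
; Perception updates for the third-person player character set the PlayerOnSight and PlayerActor blackboard keys, clearing the actor when sight is lost.
; On BeginPlay it caches the controlled BP_Enemy and binds its health component's death event to destroy that pawn.
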(event `self.ReceivePossess`
  (params (PossessedPawn :type "Pawn Object Reference"))
  (`self.RunBehaviorTree` "/Game/Blueprints/Enemy/BT_Enemy1.BT_Enemy1"))

(event `self.AIPerception.OnTargetPerceptionUpdated`
  (params (Actor :type "Actor Object Reference") (Stimulus :type "AIStimulus Structure"))
  (bind (_age _expirationage _strength _stimuluslocation _receiverlocation _tag _bsuccessfullysensed) (break `AIStimulus` Stimulus))
  (bind _asbp_third_person_character (cast `/Game/ThirdPerson/Blueprints/BP_ThirdPersonCharacter` Actor))
  (`BlackboardComponent.SetValueAsBool` (`self.Blackboard`) (`self.PlayerOnSight`) _bsuccessfullysensed)
  (if _bsuccessfullysensed
    (`BlackboardComponent.SetValueAsObject` (`self.Blackboard`) "PlayerActor" _asbp_third_person_character)
    (else
      (`BlackboardComponent.SetValueAsObject` (`self.Blackboard`) "PlayerActor" null))))

(event `self.ReceiveBeginPlay`
  (bind _asbp_enemy (cast `/Game/Blueprints/Enemy/BP_Enemy` (`self.K2_GetPawn`)))
  (set `self.ControlledEnemy` _asbp_enemy)
  (add `/Game/Blueprints/ActorComponent/Components/AC_HealthComponent.OnDeath` (`/Game/Blueprints/Enemy/BP_Enemy.AC_HealthComponent` (`self.ControlledEnemy`)) (delegate `Died`)))

(event `Died`
  (`self.K2_DestroyActor` (stale `self.ReceiveBeginPlay` _asbp_enemy)))

(fn `UserConstructionScript`)