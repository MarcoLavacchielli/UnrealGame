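; Behavior tree task that gives a BP_Enemy the next patrol waypoint location.
; On execute it casts the controlled pawn and writes the current waypoint actor's location to the BBLoc blackboard key.
; It then advances the stored index, wrapping to the first waypoint after the last, and finishes successfully.
; A failed cast stops execution before the task calls FinishExecute.
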(event `self.ReceiveExecuteAI`
  (params (OwnerController :type "AIController Object Reference") (ControlledPawn :type "Pawn Object Reference"))
  (bind _asbp_enemy (cast `/Game/Blueprints/Enemy/BP_Enemy` ControlledPawn))
  (bind _waypoints (`/Game/Blueprints/Enemy/BP_Enemy.Waypoints` _asbp_enemy))
  (`BTFunctionLibrary.SetBlackboardValueAsVector` (`self.BBLoc`) (`Actor.K2_GetActorLocation` (`|GetArrayItem` _waypoints (`self.Index`))))
  (if (>= (`self.Index`) (- (`KismetArrayLibrary.Array_Length` _waypoints) 1))
    (set `self.Index` 0)
    (else
      (`/Engine/EditorBlueprintResources/StandardMacros.IncrementInt` (`self.Index`)
        (:`  `
          _))))
  (`self.FinishExecute` true))