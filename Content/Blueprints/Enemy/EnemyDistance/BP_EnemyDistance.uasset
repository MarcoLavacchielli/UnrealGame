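; BP_EnemyDistance is the ranged enemy, which shoots bullets on attack.
; BeginPlay reads the "Range" row of DT_Enemies and applies its max health to the health component.
; StartAttack spawns BP_ABullet at BulletSpawner with a shooting montage and gunshot sound, using IsOnAttack to block re-firing until the montage completes.
; Direct-damage and collision-disabling logic remains in the graph but never runs.
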(event `self.ReceiveBeginPlay`
  (bind _returnvalue (`|GetDataTableRow` "/Game/Blueprints/Data/DT_Enemies.DT_Enemies" "Range")
    (:`then`
      (bind _output_get (set `self.EnemyData` _returnvalue))
      (`/Game/Blueprints/ActorComponent/Components/AC_HealthComponent.SetNewMaxHealth` (`self.AC_HealthComponent`) (`.MaxHealth_8_AB87AAC243B449C7E0F6C097C2719E40` (break `/Game/Blueprints/Data/S_EnemyData` _output_get)) false))))

(event `StartAttack`
  (if (not (`self.isOnAttack`))
    (set `self.isOnAttack` true)
    (`|SpawnActorFromClass` "/Game/Blueprints/Turret/source/BP_ABullet.BP_ABullet_C" (`SceneComponent.K2_GetComponentToWorld` (`self.BulletSpawner`)) "AlwaysSpawn" "MultiplyWithRoot" null null)
    (`|PlayMontage` (`self.Mesh`) "/Game/Blueprints/Enemy/EnemyDistance/Animations/AM_EnemyShooting.AM_EnemyShooting"
      (:`then`
        (`GameplayStatics.PlaySound2D` "/Game/Sfx-Music/Gunshot_Sound_Effect_Single_Shot_MP3_160K_.Gunshot_Sound_Effect_Single_Shot_MP3_160K_" 0.5 1.0 0.0 null null))
      (:`OnCompleted`
        (set `self.isOnAttack` false)
        (set `self.attackMake` false)))))

(fn `UserConstructionScript`)