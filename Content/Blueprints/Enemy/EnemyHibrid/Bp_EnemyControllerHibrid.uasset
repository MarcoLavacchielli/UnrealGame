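; AI controller for the hybrid enemy that runs its behavior tree and keeps its death persistent through the game instance.
; Perception updates on the player character set the sight flag and player reference in the Blackboard, clearing the reference when sight is lost.
; On BeginPlay it destroys a pawn whose ActorID is already recorded as destroyed.
; The health component's death event records that ID and destroys the pawn.
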(event `self.ReceivePossess`
  (params (PossessedPawn :type "Pawn Object Reference"))
  (`self.RunBehaviorTree` "/Game/Blueprints/Enemy/EnemyHibrid/BT_EnemyHibrid.BT_EnemyHibrid"))

(event `self.AIPerception.OnTargetPerceptionUpdated`
  (params (Actor :type "Actor Object Reference") (Stimulus :type "AIStimulus Structure"))
  (bind (_age _expirationage _strength _stimuluslocation _receiverlocation _tag _bsuccessfullysensed) (break `AIStimulus` Stimulus))
  (bind _asbp_third_person_character (cast `/Game/ThirdPerson/Blueprints/BP_ThirdPersonCharacter` Actor))
  (`BlackboardComponent.SetValueAsBool` (`self.Blackboard`) (`self.PlayerOnSight`) _bsuccessfullysensed)
  (if _bsuccessfullysensed
    (`BlackboardComponent.SetValueAsObject` (`self.Blackboard`) "PlayerActor" _asbp_third_person_character)
    (else
      (`BlackboardComponent.SetValueAsObject` (`self.Blackboard`) "PlayerActor" null))))

(event `self.ReceiveBeginPlay`
  (bind _asbp_enemy_hibrido (cast `/Game/Blueprints/Enemy/EnemyHibrid/BP_EnemyHibrido` (`self.K2_GetPawn`)))
  (set `self.ControlledHibridEnemy` _asbp_enemy_hibrido)
  (add `/Game/Blueprints/ActorComponent/Components/AC_HealthComponent.OnDeath` (`/Game/Blueprints/Enemy/EnemyHibrid/BP_EnemyHibrido.AC_HealthComponent` (`self.ControlledHibridEnemy`)) (delegate `Died`))
  (bind _asbp_mi_instance (cast `/Game/Blueprints/BP_GameInstanceOwn/BP_MiInstance` (`GameplayStatics.GetGameInstance`)))
  (bind _returnvalue (`/Game/Blueprints/BP_GameInstanceOwn/BP_MiInstance.Check If Already Destroyed` _asbp_mi_instance (`/Game/Blueprints/Enemy/EnemyHibrid/BP_EnemyHibrido.Actor ID` (`self.ControlledHibridEnemy`))))
  (if _returnvalue
    (`self.K2_DestroyActor` _asbp_enemy_hibrido :!label _label)))

(event `Died`
  (`self.EnemyDestroy`)
  (goto _label))

(event `EnemyDestroy`
  (bind _asbp_mi_instance (cast `/Game/Blueprints/BP_GameInstanceOwn/BP_MiInstance` (`GameplayStatics.GetGameInstance`)))
  (`/Game/Blueprints/BP_GameInstanceOwn/BP_MiInstance.DestroyItem` _asbp_mi_instance (`/Game/Blueprints/Enemy/EnemyHibrid/BP_EnemyHibrido.Actor ID` (`self.ControlledHibridEnemy`))))

(fn `UserConstructionScript`)