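; BP_EnemyHibrido is a hybrid enemy with both melee and ranged attacks, taking health and damage from the Melee row of DT_Enemies.
; StartAttack plays the attack montage, during which TrueAttack overlaps damage the player character, with a flag limiting hits to one per swing.
; StartAttackDistance spawns BP_ABullet at BulletSpawner and plays the same montage with a gunshot sound.
; Montage completion resets the attack flags; a leftover ranged-damage branch is unconnected.
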(event `self.ReceiveBeginPlay`
  (bind _returnvalue (`|GetDataTableRow` "/Game/Blueprints/Data/DT_Enemies.DT_Enemies" "Melee")
    (:`then`
      (bind _output_get (set `self.EnemyData` _returnvalue))
      (`/Game/Blueprints/ActorComponent/Components/AC_HealthComponent.SetNewMaxHealth` (`self.AC_HealthComponent`) (`.MaxHealth_8_AB87AAC243B449C7E0F6C097C2719E40` (break `/Game/Blueprints/Data/S_EnemyData` _output_get)) false)
      (`PrimitiveComponent.SetCollisionEnabled` (`self.AttackBox`) "NoCollision"))))

(event `StartAttack`
  (if (not (`self.isOnAttackMelee`))
    (set `self.isOnAttackMelee` true)
    (`|PlayMontage` (`self.Mesh`) "/Game/Blueprints/Enemy/EnemyMelee/Animations/AM_Attack.AM_Attack"
      (:`then`
        (`GameplayStatics.PlaySound2D` "/Game/Sfx-Music/Something_being_hit_-_Sound_Effect.Something_being_hit_-_Sound_Effect" 1.5 1.0 0.0 null null))
      (:`OnCompleted`
        (set `self.isOnAttackMelee` false)
        (set `self.attackMakeMelee` false)
        (set `self.isOnAttackDistance` false)))))

(event `self.TrueAttack.OnComponentBeginOverlap`
  (params (OverlappedComponent :type "PrimitiveComponent Object Reference") (OtherActor :type "Actor Object Reference") (OtherComp :type "PrimitiveComponent Object Reference") (OtherBodyIndex :type Integer) (bFromSweep :type Boolean) (SweepResult :type "HitResult Structure (by ref)"))
  (if (`self.isOnAttackMelee`)
    (bind _asbp_third_person_character (cast `/Game/ThirdPerson/Blueprints/BP_ThirdPersonCharacter` OtherActor))
    (if (`self.attackMakeMelee`)
      _
      (elif (not (== _asbp_third_person_character self))
        (`/Game/Blueprints/ActorComponent/Components/AC_HealthComponent.DecreaseHealth` (`/Game/ThirdPerson/Blueprints/BP_ThirdPersonCharacter.AC_HealthComponent` _asbp_third_person_character) (`.Damage_9_F22DB42E4A347C58A198049AC1572AC2` (break `/Game/Blueprints/Data/S_EnemyData` (`self.EnemyData`))))
        (set `self.attackMakeMelee` true)))))

(event `StartAttackDistance`
  (if (not (`self.isOnAttackDistance`))
    (set `self.isOnAttackDistance` true)
    (`|SpawnActorFromClass` "/Game/Blueprints/Turret/source/BP_ABullet.BP_ABullet_C" (`SceneComponent.K2_GetComponentToWorld` (`self.BulletSpawner`)) "AlwaysSpawn" "MultiplyWithRoot" null null)
    (`|PlayMontage` (`self.Mesh`) "/Game/Blueprints/Enemy/EnemyMelee/Animations/AM_Attack.AM_Attack"
      (:`then`
        (`GameplayStatics.PlaySound2D` "/Game/Sfx-Music/Gunshot_Sound_Effect_Single_Shot_MP3_160K_.Gunshot_Sound_Effect_Single_Shot_MP3_160K_" 0.5 1.0 0.0 null null))
      (:`OnCompleted`
        (set `self.isOnAttackDistance` false)
        (set `self.attackMakeDistance` false)
        (set `self.IsOnAttackMelee` false)))))

(fn `UserConstructionScript`)