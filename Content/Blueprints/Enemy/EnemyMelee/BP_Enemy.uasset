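; BP_Enemy is a melee enemy that plays an attack montage and damages the player character.
; On BeginPlay it reads the Melee row of DT_Enemies, sets max health on its health component and disables AttackBox collision.
; StartAttack guards against re-entry, and TrueAttack overlaps during an attack apply the row's damage to BP_ThirdPersonCharacter.
; An AttackMake flag limits damage to one hit until the montage completes.
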(event `self.ReceiveBeginPlay`
  (bind _returnvalue (`|GetDataTableRow` "/Game/Blueprints/Data/DT_Enemies.DT_Enemies" "Melee")
    (:`then`
      (bind _output_get (set `self.EnemyData` _returnvalue))
      (`/Game/Blueprints/ActorComponent/Components/AC_HealthComponent.SetNewMaxHealth` (`self.AC_HealthComponent`) (`.MaxHealth_8_AB87AAC243B449C7E0F6C097C2719E40` (break `/Game/Blueprints/Data/S_EnemyData` _output_get)) false)
      (`PrimitiveComponent.SetCollisionEnabled` (`self.AttackBox`) "NoCollision"))))

(event `StartAttack`
  (if (not (`self.isOnAttack`))
    (set `self.isOnAttack` true)
    (`|PlayMontage` (`self.Mesh`) "/Game/Blueprints/Enemy/EnemyMelee/Animations/AM_Attack.AM_Attack"
      (:`OnCompleted`
        (set `self.isOnAttack` false)
        (set `self.attackMake` false)))))

(event `self.TrueAttack.OnComponentBeginOverlap`
  (params (OverlappedComponent :type "PrimitiveComponent Object Reference") (OtherActor :type "Actor Object Reference") (OtherComp :type "PrimitiveComponent Object Reference") (OtherBodyIndex :type Integer) (bFromSweep :type Boolean) (SweepResult :type "HitResult Structure (by ref)"))
  (if (`self.isOnAttack`)
    (bind _asbp_third_person_character (cast `/Game/ThirdPerson/Blueprints/BP_ThirdPersonCharacter` OtherActor))
    (if (`self.attackMake`)
      _
      (elif (not (== _asbp_third_person_character self))
        (`/Game/Blueprints/ActorComponent/Components/AC_HealthComponent.DecreaseHealth` (`/Game/ThirdPerson/Blueprints/BP_ThirdPersonCharacter.AC_HealthComponent` _asbp_third_person_character) (`.Damage_9_F22DB42E4A347C58A198049AC1572AC2` (break `/Game/Blueprints/Data/S_EnemyData` (`self.EnemyData`))))
        (set `self.attackMake` true)))))

(fn `UserConstructionScript`)