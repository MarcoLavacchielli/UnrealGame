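; Actor component that tracks its owner's gem count and broadcasts changes through event dispatchers.
; The count resets to zero on BeginPlay, and every change fires OnGemChanged with the new total.
; Increases also fire OnGemIncrease, plus OnSecretUnlock whenever the total is at or above a hardcoded threshold.
; Decreases fire OnGemReduce only while the total stays above zero, with no clamping.
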(event `self.ReceiveBeginPlay`
  (bind _output_get (set `self.CurrentGems` 0.0))
  (`self.OnGemChanged` _output_get))

(fn `DecreaseGem`
  (params (GemAmount :type "Float (double-precision)"))
  (bind _output_get (set `self.CurrentGems` (- (`self.CurrentGems`) GemAmount)))
  (`self.OnGemChanged` _output_get)
  (if (not (<= (`self.CurrentGems`) 0.0))
    (`self.OnGemReduce`)))

(fn `IncreaseGem`
  (params (GemAmount :type "Float (double-precision)"))
  (bind _output_get (set `self.CurrentGems` (+ (`self.CurrentGems`) GemAmount)))
  (`self.OnGemChanged` _output_get)
  (if (>= (`self.CurrentGems`) 6.0)
    (`self.OnSecretUnlock`))
  (`self.OnGemIncrease`))