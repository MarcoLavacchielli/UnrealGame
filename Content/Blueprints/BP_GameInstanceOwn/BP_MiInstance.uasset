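; Game instance that saves and loads player progress in one save slot and tracks destroyed item IDs across levels.
; SaveGame writes transform, health, coins, gems, destroyed IDs and level name to a BP_LoadFiles object, re-saving after each field.
; MenuLoadGame sets a load flag and opens the saved level.
; LoadGame restores player state through its components, but copies the live destroyed list into the save object rather than reading it back.
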(event `MenuLoadGame`
  (bind _returnvalue (`GameplayStatics.GetPlayerController` 0))
  (set `self.LoadGame?` true)
  (bind _savedlevel (`self.GameLoad`))
  (`GameplayStatics.OpenLevel` (`KismetStringLibrary.Conv_StringToName` _savedlevel))
  (set `PlayerController.bShowMouseCursor` false _returnvalue)
  (`WidgetBlueprintLibrary.SetInputMode_GameOnly` _returnvalue))

(event `DestroyItem`
  (params (ItemID :type "Name (by ref)"))
  (`KismetArrayLibrary.Array_AddUnique` (`self.DestroyActors`) ItemID))

(event `ClearList`
  (`KismetArrayLibrary.Array_Clear` (`self.DestroyActors`)))

(fn `Check If Already Destroyed`
  (params (ItemID :type "Name (by ref)"))
  (returns (ReturnValue :type Boolean))
  (return (> (`KismetArrayLibrary.Array_Find` (`self.DestroyActors`) ItemID) -1)))

(fn `GameLoad`
  (returns (SavedLevel :type String))
  (bind _returnvalue (`GameplayStatics.LoadGameFromSlot` (`self.Slot Name Save`)))
  (bind _asbp_load_files (cast `/Game/Blueprints/BP_GameInstanceOwn/BP_LoadFiles` _returnvalue))
  (bind _output_get (set `self.SafeRef` _asbp_load_files))
  (return (`/Game/Blueprints/BP_GameInstanceOwn/BP_LoadFiles.SavedLevel` _output_get)))

(fn `LoadGame`
  (`|ExecutionSequence`
    (:`then_0`
      (`Actor.K2_SetActorTransform` (`self.PlayerCharacter`) (`/Game/Blueprints/BP_GameInstanceOwn/BP_LoadFiles.Transform` (`self.SafeRef`)) false false))
    (:`then_1`
      (`/Game/Blueprints/ActorComponent/Components/AC_HealthComponent.OnHealthChanged` (`/Game/ThirdPerson/Blueprints/BP_ThirdPersonCharacter.AC_HealthComponent` (`self.PlayerCharacter`)) (`/Game/Blueprints/BP_GameInstanceOwn/BP_LoadFiles.Health` (`self.SafeRef`)) (`/Game/Blueprints/ActorComponent/Components/AC_HealthComponent.MaxHealth` (`/Game/ThirdPerson/Blueprints/BP_ThirdPersonCharacter.AC_HealthComponent` (`self.PlayerCharacter`)))))
    (:`then_2`
      (`/Game/Blueprints/ActorComponent/Components/AC_CoinComponent.IncreaseCoin` (`/Game/ThirdPerson/Blueprints/BP_ThirdPersonCharacter.AC_CoinComponent` (`self.PlayerCharacter`)) (`/Game/Blueprints/BP_GameInstanceOwn/BP_LoadFiles.Coins` (`self.SafeRef`))))
    (:`then_3`
      (`/Game/Blueprints/ActorComponent/Components/AC_GemComponent.IncreaseGem` (`/Game/ThirdPerson/Blueprints/BP_ThirdPersonCharacter.AC_GemComponent` (`self.PlayerCharacter`)) (`/Game/Blueprints/BP_GameInstanceOwn/BP_LoadFiles.Gems` (`self.SafeRef`))))
    (:`then_4`
      (set `/Game/Blueprints/BP_GameInstanceOwn/BP_LoadFiles.DestroyActors` (`self.DestroyActors`) (`self.SafeRef`)))))

(fn `SaveGame`
  (bind _returnvalue (`GameplayStatics.CreateSaveGameObject` "/Game/Blueprints/BP_GameInstanceOwn/BP_LoadFiles.BP_LoadFiles_C"))
  (bind _output_get (set `self.SafeRef` _returnvalue))
  (`|ExecutionSequence`
    (:`then_0`
      (set `/Game/Blueprints/BP_GameInstanceOwn/BP_LoadFiles.Transform` (`Actor.GetTransform` (`self.PlayerCharacter`)) _output_get))
    (:`then_1`
      (set `/Game/Blueprints/BP_GameInstanceOwn/BP_LoadFiles.Health` (`/Game/Blueprints/ActorComponent/Components/AC_HealthComponent.CurrentHealth` (`/Game/ThirdPerson/Blueprints/BP_ThirdPersonCharacter.AC_HealthComponent` (`self.PlayerCharacter`))) _output_get))
    (:`then_2`
      (set `/Game/Blueprints/BP_GameInstanceOwn/BP_LoadFiles.Coins` (`/Game/Blueprints/ActorComponent/Components/AC_CoinComponent.CurrentCoin` (`/Game/ThirdPerson/Blueprints/BP_ThirdPersonCharacter.AC_CoinComponent` (`self.PlayerCharacter`))) _output_get))
    (:`then_3`
      (set `/Game/Blueprints/BP_GameInstanceOwn/BP_LoadFiles.Gems` (`/Game/Blueprints/ActorComponent/Components/AC_GemComponent.CurrentGems` (`/Game/ThirdPerson/Blueprints/BP_ThirdPersonCharacter.AC_GemComponent` (`self.PlayerCharacter`))) _output_get))
    (:`then_4`
      (set `/Game/Blueprints/BP_GameInstanceOwn/BP_LoadFiles.DestroyActors` (`self.DestroyActors`) (`self.SafeRef`))))
  (bind _returnvalue_2 (`GameplayStatics.GetCurrentLevelName` true))
  (set `/Game/Blueprints/BP_GameInstanceOwn/BP_LoadFiles.SavedLevel` _returnvalue_2 (`self.SafeRef`))
  (`GameplayStatics.SaveGameToSlot` (`self.SafeRef`) (`self.Slot Name Save`)))