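; BP_DamageBox is a trigger volume that damages the third-person player character.
; On overlap it caches the character's health component and starts a short, non-looping timer.
; When the timer fires it decreases health once by a fixed amount and plays a 2D death sound.
; Leaving the box clears the timer, cancelling any pending damage.
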(event `self.DamageBox.OnComponentBeginOverlap`
  (params (OverlappedComponent :type "PrimitiveComponent Object Reference") (OtherActor :type "Actor Object Reference") (OtherComp :type "PrimitiveComponent Object Reference") (OtherBodyIndex :type Integer) (bFromSweep :type Boolean) (SweepResult :type "HitResult Structure (by ref)"))
  (bind _asbp_third_person_character (cast `/Game/ThirdPerson/Blueprints/BP_ThirdPersonCharacter` OtherActor))
  (bind _ac_healthcomponent (`/Game/ThirdPerson/Blueprints/BP_ThirdPersonCharacter.AC_HealthComponent` _asbp_third_person_character))
  (`/Engine/EditorBlueprintResources/StandardMacros.IsValid` _ac_healthcomponent
    (:`Is Valid`
      (set `self.Ac` _ac_healthcomponent)
      (bind _returnvalue (`KismetSystemLibrary.K2_SetTimerDelegate` (delegate `DamagePlayer`) 0.1))
      (set `self.TimerReference` _returnvalue))))

(event `DamagePlayer`
  (bind _ac (`self.Ac`)
    (:`then`
      (`/Game/Blueprints/ActorComponent/Components/AC_HealthComponent.DecreaseHealth` _ac 10.0)
      (`GameplayStatics.PlaySound2D` "/Game/Sfx-Music/Muerte_de_Minecraft_-_Sonido_MP3_160K_.Muerte_de_Minecraft_-_Sonido_MP3_160K_" 1.5 1.0 0.0 null null))
    (:`else`)))

(event `self.DamageBox.OnComponentEndOverlap`
  (params (OverlappedComponent :type "PrimitiveComponent Object Reference") (OtherActor :type "Actor Object Reference") (OtherComp :type "PrimitiveComponent Object Reference") (OtherBodyIndex :type Integer))
  (cast `/Game/ThirdPerson/Blueprints/BP_ThirdPersonCharacter` OtherActor)
  (`KismetSystemLibrary.K2_ClearAndInvalidateTimerHandle` (`self.TimerReference`)))

(fn `UserConstructionScript`)